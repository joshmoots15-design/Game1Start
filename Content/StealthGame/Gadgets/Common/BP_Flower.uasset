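; BP_Flower is a pickup the player must keep watered, with messages directing them to the Light House.
; Capsule overlap increments the character's HasFlower, attaches the flower to its mesh's FlowerSocket and shows timed one-time objective hints.
; BeginPlay drains water once, then a looping timer drains it while the player's Flower value is true.
; Tick prints one-time dryness warnings at exact water levels and loads the checkpoint once water runs out.
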(event `WaterDrain`
  ;[0 0.5806 1 1 14] Water Draining
  (if (`/Game/StealthGame/Core/Characters/PlayerCharacter/BP_ThirdPersonCharacterCustom.bFlower` (`self.PlayerRef`))
    (bind _output_get (set `self.CurrentWater` (`KismetMathLibrary.FClamp` (- (`self.CurrentWater`) 2.0) 0.0 (`self.CurrentWater`)) :!label _label))
    (`KismetSystemLibrary.PrintString` (`KismetStringLibrary.Conv_DoubleToString` _output_get))))

(event `self.ReceiveBeginPlay`
  ;[0 0.5806 1 1 14] Water Draining
  (`|ExecutionSequence`
    (:`then_0`
      (bind _asbp_third_person_character_custom (cast `/Game/StealthGame/Core/Characters/PlayerCharacter/BP_ThirdPersonCharacterCustom` (`GameplayStatics.GetPlayerCharacter` 0)))
      (set `self.PlayerRef` _asbp_third_person_character_custom))
    (:`then_1`
      (`KismetSystemLibrary.K2_SetTimerDelegate` (delegate `WaterDrain`) 3.5 true)
      (goto _label))))

(event `self.Capsule.OnComponentBeginOverlap`
  (params (OverlappedComponent :type "PrimitiveComponent Object Reference") (OtherActor :type "Actor Object Reference") (OtherComp :type "PrimitiveComponent Object Reference") (OtherBodyIndex :type Integer) (bFromSweep :type Boolean) (SweepResult :type "HitResult Structure (by ref)"))
  ;[1 0.179 0 0.5] Attaching To Player Character
  (`|ExecutionSequence`
    (:`then_0`
      (bind _asbp_third_person_character_custom (cast `/Game/StealthGame/Core/Characters/PlayerCharacter/BP_ThirdPersonCharacterCustom` OtherActor))
      (set `/Game/StealthGame/Core/Characters/PlayerCharacter/BP_ThirdPersonCharacterCustom.HasFlower` (+ (`/Game/StealthGame/Core/Characters/PlayerCharacter/BP_ThirdPersonCharacterCustom.HasFlower` _asbp_third_person_character_custom) 1) _asbp_third_person_character_custom)
      (`self.K2_AttachToComponent` (`Character.Mesh` _asbp_third_person_character_custom) "FlowerSocket" "SnapToTarget" "SnapToTarget" "SnapToTarget")
      (set `self.bPickedUp` true))
    (:`then_1`
      (`/Engine/EditorBlueprintResources/StandardMacros.DoOnce` false
        (:`Completed`
          (`KismetSystemLibrary.PrintString` "Keep The Flower Alive!" true true (struct :`R` 0.991963 :`G` 0.363367 :`B` 1.0 :`A` 1.0) 5.0))))
    (:`then_2`
      (`/Engine/EditorBlueprintResources/StandardMacros.DoOnce` false
        (:`Completed`
          (`KismetSystemLibrary.Delay` 5.0)
          (`KismetSystemLibrary.PrintString` "Collect Water From Buckets, Wells, and Fountains!" true true (struct :`R` 0.21875 :`G` 0.396733 :`B` 1.0 :`A` 1.0) 5.0))))
    (:`then_3`
      (`/Engine/EditorBlueprintResources/StandardMacros.DoOnce` false
        (:`Completed`
          (`KismetSystemLibrary.Delay` 10.0)
          (`KismetSystemLibrary.PrintString` "Get to the Light House!" true true (struct :`R` 1.0 :`G` 0.149439 :`B` 0.057292 :`A` 1.0) 5.0))))))

(event `self.ReceiveTick`
  (params (DeltaSeconds :type "Float (single-precision)"))
  ;[0.842 0.001232 1 0.5] Water Draining Messages
  (`|ExecutionSequence`
    (:`then_0`
      (if (== (`self.CurrentWater`) 74.0)
        (`/Engine/EditorBlueprintResources/StandardMacros.DoOnce` false
          (:`Completed`
            (`KismetSystemLibrary.PrintString` "Getting a little dry!")))))
    (:`then_1`
      (if (== (`self.CurrentWater`) 50.0)
        (`/Engine/EditorBlueprintResources/StandardMacros.DoOnce` false
          (:`Completed`
            (`KismetSystemLibrary.PrintString` "Youre somewhat dry! !")))))
    (:`then_2`
      (if (== (`self.CurrentWater`) 24.0)
        (`/Engine/EditorBlueprintResources/StandardMacros.DoOnce` false
          (:`Completed`
            (`KismetSystemLibrary.PrintString` "Youre dry! Get Water!")))))
    (:`then_3`
      (if (== (`self.CurrentWater`) 10.0)
        (`/Engine/EditorBlueprintResources/StandardMacros.DoOnce` false
          (:`Completed`
            (`KismetSystemLibrary.PrintString` "You need water! Get it fast!")))))
    (:`then_4`
      (if (<= (`self.CurrentWater`) 0.0)
        (`/Engine/EditorBlueprintResources/StandardMacros.DoOnce` false
          (:`Completed`
            (bind _asbp_third_person_character_custom (cast `/Game/StealthGame/Core/Characters/PlayerCharacter/BP_ThirdPersonCharacterCustom` (`GameplayStatics.GetPlayerCharacter` 0)))
            (`/Game/StealthGame/Core/Characters/PlayerCharacter/BP_ThirdPersonCharacterCustom.LoadCheckpoint` _asbp_third_person_character_custom)))))))

(fn `UserConstructionScript`)