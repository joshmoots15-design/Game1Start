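; BP_WaterWell is a well gadget that tops up water on the BP_Flower actor found in the level, then becomes empty.
; Overlap with component R enables input for the player and prints the fill state.
; Pressing Interact while filled adds water, clamped to the flower's maximum, and empties the well.
; Player end overlap disables input and runs the same refill-and-empty logic without checking whether the well is filled.
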(event `self.r.OnComponentBeginOverlap`
  (params (OverlappedComponent :type "PrimitiveComponent Object Reference") (OtherActor :type "Actor Object Reference") (OtherComp :type "PrimitiveComponent Object Reference") (OtherBodyIndex :type Integer) (bFromSweep :type Boolean) (SweepResult :type "HitResult Structure (by ref)"))
  (`|ExecutionSequence`
    (:`then_0`
      (if (== OtherActor (`GameplayStatics.GetPlayerCharacter` 0))
        (`self.EnableInput` (`GameplayStatics.GetPlayerController` 0))))
    (:`then_1`
      (if (`self.WellFilled`)
        (`KismetSystemLibrary.PrintString` "The Well is full. Want to Fill Up?")
        (else
          (`KismetSystemLibrary.PrintString` "The Well Has Been Emptied" true true (struct :`R` 0.053967 :`B` 1.0 :`A` 1.0) :!label _label)
          (set `self.WellFilled` false))))))

(event `InputAction|Interact`
  (params (Key :type "Key Structure"))
  (:`Pressed`
    (if (`self.WellFilled`)
      (bind _returnvalue (`GameplayStatics.GetActorOfClass` "/Game/StealthGame/Gadgets/Common/BP_Flower.BP_Flower_C" :!label _label_2))
      (bind _output_get (set `/Game/StealthGame/Gadgets/Common/BP_Flower.CurrentWater` (`KismetMathLibrary.FClamp` (+ (`/Game/StealthGame/Gadgets/Common/BP_Flower.CurrentWater` _returnvalue) 100.0) 0.0 (`/Game/StealthGame/Gadgets/Common/BP_Flower.MaxWater` _returnvalue)) _returnvalue))
      (`KismetSystemLibrary.PrintString` (`KismetStringLibrary.Conv_DoubleToString` _output_get))
      (goto _label))))

(event `self.r.OnComponentEndOverlap`
  (params (OverlappedComponent :type "PrimitiveComponent Object Reference") (OtherActor :type "Actor Object Reference") (OtherComp :type "PrimitiveComponent Object Reference") (OtherBodyIndex :type Integer))
  (if (== OtherActor (`GameplayStatics.GetPlayerCharacter` 0))
    (`self.DisableInput` (`GameplayStatics.GetPlayerController` 0))
    (goto _label_2)))

(fn `UserConstructionScript`)