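; Stealth-game enemy AI that patrols and chases the player on sight, switching between walk and run speeds.
; PawnSensing sets a visibility flag for the custom third-person character, cleared by a two-second retriggerable delay.
; Tick prioritises chasing, otherwise using CanMove to gate target-point or random-point patrols via AIMoveTo.
; Random patrol re-issues itself after each delay, while the target-point index adds zero, so it never advances.
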(event `self.ReceiveBeginPlay`
  (`self.PatrolRandom`))

(event `self.ReceiveTick`
  (params (DeltaSeconds :type "Float (single-precision)"))
  (if (`self.bCanMove`)
    (if (`self.bPlayerVisi`)
      (`self.ChasePlayer`)
      (elif (`self.bTargetPointMovement`)
        (`self.MoveToPatrolPoint`)
        (else
          (`self.PatrolRandom`))))
    (elif (`self.bPlayerVisi`)
      (`self.ChasePlayer`))))

(event `self.PawnSensing.OnSeePawn`
  (params (Pawn :type "Pawn Object Reference"))
  (cast `/Game/StealthGame/Core/Characters/PlayerCharacter/BP_ThirdPersonCharacterCustom` Pawn
    (:`then`
      (`|ExecutionSequence`
        (:`then_0`
          (`KismetSystemLibrary.PrintString` "KABOOM")
          (set `self.bPlayerVisi` true))
        (:`then_1`
          (`KismetSystemLibrary.RetriggerableDelay` 2.0)
          (set `self.bPlayerVisi` false))))
    (:`CastFailed`
      (set `self.bPlayerVisi` false))))

(event `ChasePlayer`
  (`self.Update Walk Speed` 600.0)
  (`|AIMoveTo` self (0.0 0.0 0.0) (`GameplayStatics.GetPlayerCharacter` 0)
    (:`OnSuccess`
      (`KismetSystemLibrary.PrintString` "SHA-BAM")
      (set `self.bCanMove` true))))

(event `PatrolRandom`
  (`self.Update Walk Speed` 200.0)
  (set `self.bCanMove` false)
  (`|AIMoveTo` self (`NavigationSystemV1.K2_GetRandomReachablePointInRadius` (`self.K2_GetActorLocation`) 2000.0 null null) null :!label _label
    (:`then`
      (`KismetSystemLibrary.Delay` 3.0)
      (set `self.bCanMove` true)
      (goto _label))))

(event `MoveToPatrolPoint`
  (`self.Update Walk Speed` 200.0)
  (set `self.bCanMove` false)
  (`|AIMoveTo` self (0.0 0.0 0.0) (`|GetArrayItem` (`self.PatrolTargetPoints`) (`self.PatrolTargetIndex`))
    (:`then`
      (`self.SetNextPatrolPointIndex`)
      (`KismetSystemLibrary.Delay` 3.0)
      (set `self.bCanMove` true))))

(event `SetNextPatrolPointIndex`
  (set `self.PatrolTargetIndex` (mod (+ (`self.PatrolTargetIndex`) 0) (`KismetArrayLibrary.Array_Length` (`self.PatrolTargetPoints`)))))

(fn `Update Walk Speed`
  (params (NewWalkSpeed :type "Float (double-precision)"))
  (set `CharacterMovementComponent.MaxWalkSpeed` NewWalkSpeed (`self.CharacterMovement`)))

(fn `UserConstructionScript`)