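; A moving platform that starts when the custom third-person character overlaps it while holding at least one key, and otherwise prints a prompt to get a key.
; A timeline lerps the Platform component's relative location between the Start and End components.
; On each finish, a short delay and a FlipFlop alternate reversing and replaying the timeline, so the platform keeps shuttling back and forth.
; The key count is only checked, not decremented.
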(event `self.ReceiveActorBeginOverlap`
  (params (OtherActor :type "Actor Object Reference"))
  (bind _asbp_third_person_character_custom (cast `/Game/StealthGame/Core/Characters/PlayerCharacter/BP_ThirdPersonCharacterCustom` OtherActor))
  (if (> (`/Game/StealthGame/Core/Characters/PlayerCharacter/BP_ThirdPersonCharacterCustom.Key Count` _asbp_third_person_character_custom) 0)
    (bind (_direction _floattrack) (`Timeline|Timeline` :!label _label)
      (:`Update`
        (`SceneComponent.K2_SetRelativeLocation` (`self.Platform`) (`KismetMathLibrary.VLerp` (`SceneComponent.RelativeLocation` (`self.Start`)) (`SceneComponent.RelativeLocation` (`self.End`)) _floattrack) false false))
      (:`Finished`
        (`KismetSystemLibrary.Delay` 2.0)
        (`/Engine/EditorBlueprintResources/StandardMacros.FlipFlop` ; If A, Reverse from End\nif B, Start from Beginning
          (:`A`
            (goto _label :!via `ReverseFromEnd`))
          (:`B`
            (goto _label :!via `PlayFromStart`)))))
    (else
      (`KismetSystemLibrary.PrintString` "get a key!"))))

(fn `UserConstructionScript`)