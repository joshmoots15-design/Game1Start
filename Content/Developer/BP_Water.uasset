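; BP_Water is a water pickup that refills the flower's water when the player character touches it.
; Overlap on its Box checks for BP_ThirdPersonCharacterCustom, then finds a BP_Flower through GetActorOfClass rather than a stored reference.
; It adds a random amount to that flower's CurrentWater, clamped to MaxWater, then destroys itself and prints the new level.
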(event `self.Box.OnComponentBeginOverlap`
  (params (OverlappedComponent :type "PrimitiveComponent Object Reference") (OtherActor :type "Actor Object Reference") (OtherComp :type "PrimitiveComponent Object Reference") (OtherBodyIndex :type Integer) (bFromSweep :type Boolean) (SweepResult :type "HitResult Structure (by ref)"))
  (cast `/Game/StealthGame/Core/Characters/PlayerCharacter/BP_ThirdPersonCharacterCustom` OtherActor)
  (bind _returnvalue (`GameplayStatics.GetActorOfClass` "/Game/Developer/BP_Flower.BP_Flower_C"))
  (bind _output_get (set `/Game/Developer/BP_Flower.CurrentWater` (`KismetMathLibrary.FClamp` (+ (`/Game/Developer/BP_Flower.CurrentWater` _returnvalue) (`KismetMathLibrary.RandomFloatInRange` 50.0 100.0)) 0.0 (`/Game/Developer/BP_Flower.MaxWater` _returnvalue)) _returnvalue))
  (`self.K2_DestroyActor`)
  (`KismetSystemLibrary.PrintString` (`KismetStringLibrary.Conv_DoubleToString` _output_get)))

(fn `UserConstructionScript`)