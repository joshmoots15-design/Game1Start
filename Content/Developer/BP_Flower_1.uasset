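; Pickup flower that the player can carry and that loses water over time until it dies.
; Capsule overlap asks BP_ThirdPersonCharacterCustom to pick it up, while CustomEvent marks it picked up and attaches it to the supplied mesh's FlowerSocket.
; BeginDrain, not called within this Blueprint, runs a retriggerable-delay loop that decrements CurrentWater each second once carried, printing debug messages.
; An unwired older pickup chain remains unused.
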(event `BeginDrain`
  (if (> (`self.bIsPickedUp`) 0)
    (if (> (`self.CurrentWater`) 0.0) :!label _label
      (set `self.CurrentWater` (- (`self.CurrentWater`) 1))
      (`KismetSystemLibrary.PrintString` "Losing Water")
      (`KismetSystemLibrary.RetriggerableDelay` 1.0)
      (goto _label)
      (else
        (`KismetSystemLibrary.PrintString` "The Flower Is Dead :(")))))

(event `self.Capsule.OnComponentBeginOverlap`
  (params (OverlappedComponent :type "PrimitiveComponent Object Reference") (OtherActor :type "Actor Object Reference") (OtherComp :type "PrimitiveComponent Object Reference") (OtherBodyIndex :type Integer) (bFromSweep :type Boolean) (SweepResult :type "HitResult Structure (by ref)"))
  ;[1 0.5395 0.008568] Pickup Rock
  (if (not (`self.bIsPickedUp`))
    (bind _asbp_third_person_character_custom (cast `/Game/StealthGame/Core/Characters/PlayerCharacter/BP_ThirdPersonCharacterCustom` OtherActor)) ; Make sure the overlapping actor is the player
    (`/Game/StealthGame/Core/Characters/PlayerCharacter/BP_ThirdPersonCharacterCustom.TryToPickUp` _asbp_third_person_character_custom null) ; Call TryToPickUp Event from BP_ThirdPersonCharacterCustom
  ))

(event `CustomEvent`
  (params (ParentMesh :type "SkeletalMeshComponent Object Reference"))
  ;[1 0.5395 0.008568] Pickup Rock
  (set `self.bIsPickedUp` true)
  (`SceneComponent.K2_AttachToComponent` (`self.DefaultSceneRoot`) ParentMesh "FlowerSocket" "SnapToTarget" "KeepRelative" "KeepRelative" true) ; Snap the rock to the player's righ hand
  (set `self.bIsPickedUp` true))

(fn `UserConstructionScript`)